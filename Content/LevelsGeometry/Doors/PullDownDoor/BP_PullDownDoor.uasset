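; BP_PullDownDoor is a vertically sliding door that, while fixed, can be pulled down and rises again on a timer.
; Separate timelines drive the door mesh's relative Z for normal and broken motion.
; When broken, DownEvent and UpEvent chain each other so the door cycles continuously until fixed.
; Its KillBox catches BP_Character while broken, using a DoOnce gate to send death and delayed spawn messages.
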(event OnComponentBeginOverlap(KillBox)
  (params (OverlappedComponent :type Primitive%20Component%20Object%20Reference) (OtherActor :type Actor%20Object%20Reference) (OtherComp :type Primitive%20Component%20Object%20Reference) (OtherBodyIndex :type Integer) (bFromSweep :type Boolean) (SweepResult :type Hit%20Result%20Structure%20%28by%20ref%29))
  (bind _asbp_character (Utilities|Casting|CastToBP_Character OtherActor))
  (bind _output_get (Variables|Default|SetCharRef _asbp_character))
  (Utilities|FlowControl|Sequence
    (:then_0
      (if (Variables|Default|GetReset)
        (goto _label Reset)))
    (:then_1
      (if (not (Variables|Default|GetIsReady))
        (Utilities|FlowControl|DoOnce false :!label _label
          (:Completed
            (Variables|Default|SetReset false)
            (Class|BPIDeath|Death(Message) _output_get)
            (Utilities|FlowControl|Delay 1.0)
            (Class|BPISpawn|Spawn(Message) _output_get)
            (Variables|Default|SetReset true)))))))

(event Custom|PullUpEvent
  (bind _pullup (Timeline|Up Play)
    (:Update
      (Transformation|SetRelativeLocation (Variables|Default|GetPullDownDoor) (Math|Vector|MakeVector 0.0 0.0 _pullup) false false))
    (:Finished
      (Variables|Default|SetIsOpened true))))

(event Custom|UpEvent
  (if (not (Variables|Default|GetIsReady))
    (bind _pullup (Timeline|UpBroken PlayFromStart)
      (:Update
        (Transformation|SetRelativeLocation (Variables|Default|GetPullDownDoor) (Math|Vector|MakeVector 0.0 0.0 _pullup) false false))
      (:Finished
        (CallFunction|DownEvent)))))

(event Custom|DownEvent
  (if (not (Variables|Default|GetIsReady))
    (bind _pulldown (Timeline|DownBroken PlayFromStart)
      (:Update
        (Transformation|SetRelativeLocation (Variables|Default|GetPullDownDoor) (Math|Vector|MakeVector 0.0 0.0 _pulldown) false false))
      (:Finished
        (CallFunction|UpEvent)))))

(event EventBeginPlay)

(event Collision|EventActorBeginOverlap
  (params (OtherActor :type Actor%20Object%20Reference)))

(event EventTick
  (params (DeltaSeconds :type Float%20%28single-precision%29)))

(event EventPullDown
  (if (Variables|Default|GetIsReady)
    (if (Variables|Default|GetIsOpened)
      (bind _pulldown (Timeline|Down Play)
        (:Update
          (Transformation|SetRelativeLocation (Variables|Default|GetPullDownDoor) (Math|Vector|MakeVector 0.0 0.0 _pulldown) false false)
          (Utilities|Time|SetTimerbyEvent (delegate Custom|PullUpEvent) 5.0))
        (:Finished
          (Variables|Default|SetIsOpened false))))))

(event EventPullDownBroken
  (Variables|Default|SetIsReady false)
  (CallFunction|DownEvent))

(event EventPullDownFixed
  (Variables|Default|SetIsReady true))

(fn ConstructionScript)