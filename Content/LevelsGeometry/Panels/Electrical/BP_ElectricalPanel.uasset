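; BP_ElectricalPanel is an interactable electrical panel whose two doors swing open and which flags the player's first-day task as done.
; The Interaction event plays two timelines that set the yaw of Arrow and Arrow1, which appear to act as door pivots.
; The same event casts the player character to BP_Character and sets its 1DayTask flag, without waiting for the door animations to finish.
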(event EventBeginPlay)

(event Collision|EventActorBeginOverlap
  (params (OtherActor :type Actor%20Object%20Reference)))

(event EventTick
  (params (DeltaSeconds :type Float%20%28single-precision%29)))

(event EventInteraction
  (Utilities|FlowControl|Sequence
    (:then_0
      (bind _doorrotation (Timeline|DoorRotate Play)
        (:Update
          (Transformation|SetRelativeRotation (Variables|Default|GetArrow) (Math|Rotator|MakeRotator 0.0 0.0 _doorrotation) false false))))
    (:then_1
      (bind _doorrotation_2 (Timeline|Door2Rotate Play)
        (:Update
          (Transformation|SetRelativeRotation (Variables|Default|GetArrow1) (Math|Rotator|MakeRotator 0.0 0.0 _doorrotation_2) false false))))
    (:then_2
      (bind _asbp_character (Utilities|Casting|CastToBP_Character (Game|GetPlayerCharacter 0)))
      (bind _output_get (Variables|Default|SetCharRef _asbp_character))
      (Variables|/Game/World/Character/Blueprints/BP_Character.BP_Character_C|Set1DayTask _output_get true))))

(fn ConstructionScript)