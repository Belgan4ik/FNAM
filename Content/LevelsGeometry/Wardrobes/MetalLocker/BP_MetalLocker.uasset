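; Metal locker the player can hide in, entered and left through the Interaction event.
; A gate and player input open on BP_Character overlap with the Box, close on end overlap, and reopen a Cooldown after each interaction.
; ToggleHide flips the character's visibility and collision and blends the camera between locker and character.
; In parallel, the Openclose timeline swings the Arrow's yaw between CloseAngle and OpenAngle.
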(event OnComponentBeginOverlap(Box)
  (params (OverlappedComponent :type Primitive%20Component%20Object%20Reference) (OtherActor :type Actor%20Object%20Reference) (OtherComp :type Primitive%20Component%20Object%20Reference) (OtherBodyIndex :type Integer) (bFromSweep :type Boolean) (SweepResult :type Hit%20Result%20Structure%20%28by%20ref%29))
  (bind _asbp_character (Utilities|Casting|CastToBP_Character OtherActor))
  (Variables|Default|SetCharRef _asbp_character)
  (Input|EnableInput (Game|GetPlayerController 0))
  (Utilities|FlowControl|Gate true) ; enters at Open
)

(event OnComponentEndOverlap(Box)
  (params (OverlappedComponent :type Primitive%20Component%20Object%20Reference) (OtherActor :type Actor%20Object%20Reference) (OtherComp :type Primitive%20Component%20Object%20Reference) (OtherBodyIndex :type Integer))
  (bind _returnvalue (Game|GetPlayerController 0))
  (bind _asbp_character (Utilities|Casting|CastToBP_Character OtherActor))
  (Variables|Default|SetCharRef _asbp_character)
  (Input|DisableInput _returnvalue)
  (Utilities|FlowControl|Gate true) ; enters at Close
)

(event EventBeginPlay)

(event Collision|EventActorBeginOverlap
  (params (OtherActor :type Actor%20Object%20Reference)))

(event EventTick
  (params (DeltaSeconds :type Float%20%28single-precision%29)))

(event EventInteraction
  (Utilities|FlowControl|Gate true :!label _label
    (:Exit
      (Utilities|FlowControl|Sequence
        (:then_0
          (CallFunction|ToggleHide)
          (Utilities|FlowControl|Delay (Variables|Default|GetCooldown))
          (Input|EnableInput (Game|GetPlayerController 0))
          (goto _label Open))
        (:then_1
          (bind _open_close (Timeline|open/close Play)
            (:Update
              (Transformation|SetRelativeRotation (Variables|Default|GetArrow) (Math|Rotator|MakeRotator 0.0 0.0 (Math|Float|Lerp (Variables|Default|GetCloseAngle) (Variables|Default|GetOpenAngle) _open_close)) false false))))))))

(fn ConstructionScript)

(fn ToggleHide
  (bind _returnvalue (Game|GetPlayerController 0))
  (bind _charref (Variables|Default|GetCharRef))
  (bind _blend_time (Variables|Default|GetBlend%20Time))
  (if (Variables|Default|GetIsHiding)
    (Variables|Default|SetIsHiding false)
    (Rendering|SetActorHiddenInGame _charref false)
    (Collision|SetActorEnableCollision _charref true)
    (Game|Player|SetViewTargetwithBlend _returnvalue _charref _blend_time "VTBlend_Linear" 0.0 false)
    (else
      (Variables|Default|SetIsHiding true)
      (Rendering|SetActorHiddenInGame _charref true)
      (Collision|SetActorEnableCollision _charref false)
      (Game|Player|SetViewTargetwithBlend _returnvalue self _blend_time "VTBlend_Linear" 0.0 false))))