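; BP_Bed1 is an interactable bed that lets the player sleep for a set time.
; On Interaction it blends the view to the bed, disables the player character's input and shows a sleep message on the UI_HUD widget.
; After a SleepTime delay it blends the view back to the character and restores input.
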(event EventBeginPlay)

(event Collision|EventActorBeginOverlap
  (params (OtherActor :type Actor%20Object%20Reference)))

(event EventTick
  (params (DeltaSeconds :type Float%20%28single-precision%29)))

(event EventInteraction
  (bind _returnvalue (Game|GetPlayerController 0))
  (bind _returnvalue_2 (Game|GetPlayerController 0))
  (bind _asbp_character (Utilities|Casting|CastToBP_Character (Game|GetPlayerCharacter 0)))
  (bind _output_get (Variables|Default|SetCharRef _asbp_character))
  (Game|Player|SetViewTargetwithBlend _returnvalue self (Variables|Default|GetBlend%20Time) "VTBlend_Linear" 0.0 false)
  (Input|DisableInput _output_get _returnvalue)
  (bind _foundwidgets (Widget|GetAllWidgetsOfClass "/Game/World/Character/HUD/UI_HUD.UI_HUD_C" true))
  (Class|BPISleep|Sleep(Message) _foundwidgets)
  (Utilities|FlowControl|Delay (Variables|Default|GetSleep%20Time))
  (Game|Player|SetViewTargetwithBlend _returnvalue_2 (Variables|Default|GetCharRef) (Variables|Default|GetBlend%20Time) "VTBlend_Linear" 0.0 false)
  (Input|EnableInput (Variables|Default|GetCharRef) _returnvalue_2))

(fn ConstructionScript)