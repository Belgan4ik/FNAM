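; BP_MetalTable is an interactable metal table with two boxes, apparently drawers, that slide open and closed along local Y via timelines.
; A single interaction alternates through a FlipFlop, opening one box while reversing the other.
; Repeated interactions reverse the last opened box once a timeline has finished and set IsReady.
; InteractionReleased uses a short retriggerable delay to reset the click count and ready flag, forming a multi-click window.
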(event Custom|PlayBox2Event
  (bind _open_close (Timeline|open/close%20box2 Play)
    (:Update
      (Transformation|SetRelativeLocation (Variables|Default|GetMetalTableBox2) (Math|Vector|MakeVector -58.0 _open_close -5.0) false false))
    (:Finished
      (Variables|Default|SetIsReady true))))

(event Custom|ReverseBox2Event
  (bind _open_close (Timeline|open/close%20box2 Reverse)
    (:Update
      (Transformation|SetRelativeLocation (Variables|Default|GetMetalTableBox2) (Math|Vector|MakeVector -58.0 _open_close -5.0) false false))
    (:Finished
      (Variables|Default|SetIsReady true))))

(event Custom|PlayBox1Event
  (bind _open_close (Timeline|open/close%20box1 Play)
    (:Update
      (Transformation|SetRelativeLocation (Variables|Default|GetMetalTableBox1) (Math|Vector|MakeVector -58.0 _open_close 2e+01) false false))
    (:Finished
      (Variables|Default|SetIsReady true))))

(event Custom|ReverseBox1Event
  (bind _open_close (Timeline|open/close%20box1 Reverse)
    (:Update
      (Transformation|SetRelativeLocation (Variables|Default|GetMetalTableBox1) (Math|Vector|MakeVector -58.0 _open_close 2e+01) false false))
    (:Finished
      (Variables|Default|SetIsReady true))))

(event EventInteraction
  (bind _result (Math|Integer|IncrementInt (Variables|Default|GetClickCount))
    (:%20%20
      (if (>= _result 2)
        (if (Variables|Default|GetIsReady)
          (if (stale _isa)
            (CallFunction|ReverseBox1Event)
            (else
              (CallFunction|ReverseBox2Event))))
        (elif (not (Variables|Default|GetIsReady))
          (bind _isa (Utilities|FlowControl|FlipFlop)
            (:A
              (Utilities|FlowControl|Sequence
                (:then_0
                  (CallFunction|PlayBox1Event))
                (:then_1
                  (CallFunction|ReverseBox2Event))))
            (:B
              (Utilities|FlowControl|Sequence
                (:then_0
                  (CallFunction|PlayBox2Event))
                (:then_1
                  (CallFunction|ReverseBox1Event))))))))))

(event EventInteractionReleased
  (Utilities|FlowControl|RetriggerableDelay 0.4)
  (Variables|Default|SetClickCount 0)
  (Variables|Default|SetIsReady false))

(fn ConstructionScript)