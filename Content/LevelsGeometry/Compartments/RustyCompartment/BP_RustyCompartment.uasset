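; BP_RustyCompartment is the blueprint for a rusty compartment level section that gates a pull-down door behind a gear puzzle.
; Its GearCheck event walks a nested chain of readiness flags for big, mid and small gears.
; When every gear is ready, it finds the BP_PullDownDoor actors in the level and sends them the PullDownFixedMessage.
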(event EventGearCheck
  (if (Variables|Default|GetIsReadyBigGearGeneral)
    (if (Variables|Default|GetIsReadyMidGear1)
      (if (Variables|Default|GetIsReadySmallGear1)
        (if (Variables|Default|GetIsReadyBigGearCentral)
          (if (Variables|Default|GetIsReadySmallGear2)
            (if (Variables|Default|GetIsReadySmallGear3)
              (if (Variables|Default|GetIsReadySmallGear4)
                (if (Variables|Default|GetIsReadyMidGear2)
                  (if (Variables|Default|GetIsReadyBigGearEnd)
                    (bind _outactors (Actor|GetAllActorsOfClass "/Game/LevelsGeometry/Doors/PullDownDoor/BP_PullDownDoor.BP_PullDownDoor_C"))
                    (Class|BPIPullDownDoorFixed|PullDownFixed(Message) _outactors)))))))))))

(fn ConstructionScript)