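; Gear socket for small gear slot 4 in the Rusty Compartment puzzle, where the player places or picks up gears.
; With the inventory open, Interaction picks up the set gear or spawns the equipped item at the Sphere, decrementing its count.
; Placement starts gear rotation, sets the compartment's readiness flag from a tag match, then triggers its gear check.
; Separate events spawn a BP_MidGear directly or destroy the current gear.
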(event Custom|GearSetEvent
  (CallFunction|SmallGearSetEvent)
  (Class|BPIGearCheck|GearCheck(Message) (Variables|Default|GetRustyCompartmentRef)))

(event Custom|SmallGearSetEvent
  (bind _rustycompartmentref (Variables|Default|GetRustyCompartmentRef))
  ;[1 1 1] SmallGear Set
  (if (Actor|ActorHasTag (Variables|Default|GetGearRef) (Variables|Default|GetGearTag))
    (Variables|/Game/LevelsGeometry/Compartments/RustyCompartment/BP_RustyCompartment.BP_RustyCompartment_C|SetIsReadySmallGear4 _rustycompartmentref true)
    (else
      (Variables|/Game/LevelsGeometry/Compartments/RustyCompartment/BP_RustyCompartment.BP_RustyCompartment_C|SetIsReadySmallGear4 _rustycompartmentref false))))

(event EventBeginPlay
  (bind _outactors (Actor|GetAllActorsOfClass "/Game/LevelsGeometry/Compartments/RustyCompartment/BP_RustyCompartment.BP_RustyCompartment_C"))
  (Variables|Default|SetRustyCompartmentRef (Utilities|Array|Get(acopy) _outactors)))

(event EventGearClean
  (Actor|DestroyActor (Variables|Default|GetGearRef))
  (Variables|Default|SetGearSet false))

(event EventGearSpawn
  (bind _sphere (Variables|Default|GetSphere))
  ;[1 1 1] Gear Spawn
  (if (not (Variables|Default|GetGearSet))
    (bind _returnvalue (Game|SpawnActorfromClass "/Game/LevelsGeometry/Gears/RustyGears/MidGear/BP_MidGear.BP_MidGear_C" (Math|Transform|MakeTransform (Transformation|GetWorldLocation _sphere) (Transformation|GetWorldRotation _sphere) "1,1,1") "Undefined" 0 0))
    (bind _output_get (Variables|Default|SetGearRef _returnvalue))
    (Variables|Default|SetGearSet true)
    (Collision|SetActorEnableCollision _output_get false)
    (Class|BPIGearRotation|GearRotation(Message) _output_get)))

(event EventInteraction
  (bind _sphere (Variables|Default|GetSphere))
  ;[1 1 1] Pick/Set Gear
  (bind _asbp_character (Utilities|Casting|CastToBP_Character (Game|GetPlayerCharacter 0)))
  (bind _output_get (Variables|Default|SetCharRef _asbp_character))
  (if (Variables|/Game/World/Character/Blueprints/BP_Character.BP_Character_C|GetInventoryOpen _output_get)
    (if (Variables|Default|GetGearSet)
      (Class|BPIGearPick|GearPick(Message) (Variables|Default|GetGearRef))
      (Variables|Default|SetGearSet false)
      (elif (>= (- (Utilities|Array|Get(acopy) (Variables|/Game/World/Character/Blueprints/BP_Character.BP_Character_C|GetItemCount _output_get) (Utilities|Array|FindItem (Variables|/Game/World/Character/Blueprints/BP_Character.BP_Character_C|GetInventory _output_get) (Utilities|Array|Get(acopy) (Variables|/Game/World/Character/Blueprints/BP_Character.BP_Character_C|GetInventory _output_get) (Variables|/Game/World/Character/Blueprints/BP_Character.BP_Character_C|GetCurrentlyEquippedInventory _output_get)))) 1) 0)
        (if (Utilities|Array|ContainsItem (Variables|/Game/World/Character/Blueprints/BP_Character.BP_Character_C|GetInventory _output_get) (Utilities|Array|Get(acopy) (Variables|/Game/World/Character/Blueprints/BP_Character.BP_Character_C|GetInventory _output_get) (Variables|/Game/World/Character/Blueprints/BP_Character.BP_Character_C|GetCurrentlyEquippedInventory _output_get)))
          (Utilities|Array|SetArrayElem (Variables|/Game/World/Character/Blueprints/BP_Character.BP_Character_C|GetItemCount _output_get) (Utilities|Array|FindItem (Variables|/Game/World/Character/Blueprints/BP_Character.BP_Character_C|GetInventory _output_get) (Utilities|Array|Get(acopy) (Variables|/Game/World/Character/Blueprints/BP_Character.BP_Character_C|GetInventory _output_get) (Variables|/Game/World/Character/Blueprints/BP_Character.BP_Character_C|GetCurrentlyEquippedInventory _output_get))) (- (Utilities|Array|Get(acopy) (Variables|/Game/World/Character/Blueprints/BP_Character.BP_Character_C|GetItemCount _output_get) (Utilities|Array|FindItem (Variables|/Game/World/Character/Blueprints/BP_Character.BP_Character_C|GetInventory _output_get) (Utilities|Array|Get(acopy) (Variables|/Game/World/Character/Blueprints/BP_Character.BP_Character_C|GetInventory _output_get) (Variables|/Game/World/Character/Blueprints/BP_Character.BP_Character_C|GetCurrentlyEquippedInventory _output_get)))) 1))
          (else
            (Utilities|Array|Add (Variables|/Game/World/Character/Blueprints/BP_Character.BP_Character_C|GetInventory _output_get) (Utilities|Array|Get(acopy) (Variables|/Game/World/Character/Blueprints/BP_Character.BP_Character_C|GetInventory _output_get) (Variables|/Game/World/Character/Blueprints/BP_Character.BP_Character_C|GetCurrentlyEquippedInventory _output_get)))
            (Utilities|Array|Add (Variables|/Game/World/Character/Blueprints/BP_Character.BP_Character_C|GetItemCount _output_get) 1)))
        (bind _returnvalue (Game|SpawnActorfromClass (Utilities|Array|Get(acopy) (Variables|/Game/World/Character/Blueprints/BP_Character.BP_Character_C|GetInventory _output_get) (Variables|/Game/World/Character/Blueprints/BP_Character.BP_Character_C|GetCurrentlyEquippedInventory _output_get)) (Math|Transform|MakeTransform (Transformation|GetWorldLocation _sphere) (Transformation|GetWorldRotation _sphere) "1,1,1") "Undefined" 0 0))
        (bind _output_get_2 (Variables|Default|SetGearRef _returnvalue))
        (Variables|Default|SetGearSet true)
        (Collision|SetActorEnableCollision _returnvalue false)
        (Class|BPIInventoryUpdate|InventoryUpdate(Message) (Variables|Default|GetCharRef))
        (Class|BPIGearRotation|GearRotation(Message) _output_get_2)
        (CallFunction|GearSetEvent)))))

(fn ConstructionScript)