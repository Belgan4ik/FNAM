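; BP_MidGear is a rusty gear actor for level geometry that rotates on demand.
; GearRotationStart plays the Rotate timeline, which feeds its track into the pitch of the Gear component's relative rotation.
; GearRotationStop halts the timeline; BeginPlay, overlap and Tick are disabled, so spinning relies on those two events being called.
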(event EventBeginPlay
  (|CallParentFunction) ; This node is disabled and will not be called.\nDrag off pins to build functionality.
)

(event Collision|EventActorBeginOverlap
  (params (OtherActor :type Actor%20Object%20Reference))
  (|CallParentFunction OtherActor) ; This node is disabled and will not be called.\nDrag off pins to build functionality.
)

(event EventTick
  (params (DeltaSeconds :type Float%20%28single-precision%29))
  (|CallParentFunction DeltaSeconds) ; This node is disabled and will not be called.\nDrag off pins to build functionality.
)

(event EventGearRotationStart
  (bind _rotate (Timeline|rotate Play)
    (:Update
      (Transformation|SetRelativeRotation (Variables|Default|GetGear) (Math|Rotator|MakeRotator 0.0 _rotate 0.0) false false))))

(event EventGearRotationStop
  (bind _rotate (Timeline|rotate Stop)
    (:Update
      (Transformation|SetRelativeRotation (Variables|Default|GetGear) (Math|Rotator|MakeRotator 0.0 _rotate 0.0) false false))))

(fn ConstructionScript
  (|CallParentFunction))