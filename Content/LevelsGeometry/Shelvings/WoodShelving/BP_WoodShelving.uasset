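; BP_WoodShelving is an interactable wooden shelving unit whose two doors swing open and closed.
; Each Interaction event triggers both doors in sequence, with a separate FlipFlop per door alternating between playing and reversing its timeline.
; The two timelines drive the yaw of Arrow1 and Arrow2, which act as the door pivots.
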(event EventInteraction
  (Utilities|FlowControl|Sequence
    (:then_0
      (Utilities|FlowControl|FlipFlop
        (:A
          (bind _open_close_door (Timeline|open/close%20door1 Play)
            (:Update
              (Transformation|SetRelativeRotation (Variables|Default|GetArrow1) (Math|Rotator|MakeRotator 0.0 0.0 _open_close_door) false false))))
        (:B
          (Timeline|open/close%20door1 Reverse))))
    (:then_1
      (Utilities|FlowControl|FlipFlop
        (:A
          (bind _open_close_door_2 (Timeline|open/close%20door2 Play)
            (:Update
              (Transformation|SetRelativeRotation (Variables|Default|GetArrow2) (Math|Rotator|MakeRotator 0.0 0.0 _open_close_door_2) false false))))
        (:B
          (Timeline|open/close%20door2 Reverse))))))

(fn ConstructionScript)