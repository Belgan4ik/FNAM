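; BP_Time is the in-game clock that tracks days and hours.
; A TimeSpan timeline, with play rate set by Speed and kicked by a looping timer, supplies seconds that become a Timespan; on finish it restarts and increments Days.
; Each update looks up HUD widgets, BP_Clock actors and the player character, sending day messages to HUD and character and hour messages to HUD and clocks.
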(event Custom|TimeLoopEvent
  (bind _second (Timeline|TimeSpan PlayFromStart)
    (:Update
      (Variables|Default|SetSecond _second)
      (bind _output_get (Variables|Default|SetTime (Math|Timespan|MakeTimespan (Variables|Default|GetDays) 0 0 (Math|Float|Truncate (Variables|Default|GetSecond)))))
      (bind _output_get_2 (Variables|Default|SetHours (.Hours (Math|Timespan|BreakTimespan _output_get))))
      (bind _output_get_3 (Variables|Default|SetDays (.Days (Math|Timespan|BreakTimespan _output_get))))
      (bind _foundwidgets (Widget|GetAllWidgetsOfClass "/Game/World/Character/HUD/UI_HUD.UI_HUD_C" true))
      (bind _outactors (Actor|GetAllActorsOfClass "/Game/LevelsGeometry/Clocks/BP_Clock.BP_Clock_C"))
      (bind _asbp_character (Utilities|Casting|CastToBP_Character (Game|GetPlayerCharacter 0)))
      (bind _output_get_4 (Variables|Default|SetCharRef _asbp_character))
      (Utilities|FlowControl|Sequence
        (:then_0
          (Class|BPIDays|Day(Message) _foundwidgets _output_get_3)
          (Class|BPIDays|Day(Message) _output_get_4 _output_get_3))
        (:then_1
          (Class|BPIHours|Hour(Message) _foundwidgets _output_get_2)
          (Class|BPIHours|Hour(Message) _outactors _output_get_2))))
    (:Finished
      (CallFunction|TimeLoopEvent)
      (Variables|Default|SetDays (+ (Variables|Default|GetDays) 1)))))

(event Custom|TimeEvent
  (bind _second (Timeline|TimeSpan Play)
    (:Update
      (Variables|Default|SetSecond _second)
      (bind _output_get (Variables|Default|SetTime (Math|Timespan|MakeTimespan (Variables|Default|GetDays) 0 0 (Math|Float|Truncate (Variables|Default|GetSecond)))))
      (bind _output_get_2 (Variables|Default|SetHours (.Hours (Math|Timespan|BreakTimespan _output_get))))
      (bind _output_get_3 (Variables|Default|SetDays (.Days (Math|Timespan|BreakTimespan _output_get))))
      (bind _foundwidgets (Widget|GetAllWidgetsOfClass "/Game/World/Character/HUD/UI_HUD.UI_HUD_C" true))
      (bind _outactors (Actor|GetAllActorsOfClass "/Game/LevelsGeometry/Clocks/BP_Clock.BP_Clock_C"))
      (bind _asbp_character (Utilities|Casting|CastToBP_Character (Game|GetPlayerCharacter 0)))
      (bind _output_get_4 (Variables|Default|SetCharRef _asbp_character))
      (Utilities|FlowControl|Sequence
        (:then_0
          (Class|BPIDays|Day(Message) _foundwidgets _output_get_3)
          (Class|BPIDays|Day(Message) _output_get_4 _output_get_3))
        (:then_1
          (Class|BPIHours|Hour(Message) _foundwidgets _output_get_2)
          (Class|BPIHours|Hour(Message) _outactors _output_get_2))))
    (:Finished
      (CallFunction|TimeLoopEvent)
      (Variables|Default|SetDays (+ (Variables|Default|GetDays) 1)))))

(event EventBeginPlay
  (Variables|Default|SetDays 1)
  (Utilities|Time|SetTimerbyEvent (delegate Custom|TimeEvent) 0.5 true))

(event EventTimeReset
  (bind _second (Timeline|TimeSpan SetNewTime)
    (:Update
      (Variables|Default|SetSecond _second)
      (bind _output_get (Variables|Default|SetTime (Math|Timespan|MakeTimespan (Variables|Default|GetDays) 0 0 (Math|Float|Truncate (Variables|Default|GetSecond)))))
      (bind _output_get_2 (Variables|Default|SetHours (.Hours (Math|Timespan|BreakTimespan _output_get))))
      (bind _output_get_3 (Variables|Default|SetDays (.Days (Math|Timespan|BreakTimespan _output_get))))
      (bind _foundwidgets (Widget|GetAllWidgetsOfClass "/Game/World/Character/HUD/UI_HUD.UI_HUD_C" true))
      (bind _outactors (Actor|GetAllActorsOfClass "/Game/LevelsGeometry/Clocks/BP_Clock.BP_Clock_C"))
      (bind _asbp_character (Utilities|Casting|CastToBP_Character (Game|GetPlayerCharacter 0)))
      (bind _output_get_4 (Variables|Default|SetCharRef _asbp_character))
      (Utilities|FlowControl|Sequence
        (:then_0
          (Class|BPIDays|Day(Message) _foundwidgets _output_get_3)
          (Class|BPIDays|Day(Message) _output_get_4 _output_get_3))
        (:then_1
          (Class|BPIHours|Hour(Message) _foundwidgets _output_get_2)
          (Class|BPIHours|Hour(Message) _outactors _output_get_2))))
    (:Finished
      (CallFunction|TimeLoopEvent)
      (Variables|Default|SetDays (+ (Variables|Default|GetDays) 1)))))

(fn ConstructionScript
  (Components|Timeline|SetPlayRate (Variables|Default|GetTimeSpan) (Variables|Default|GetSpeed)))