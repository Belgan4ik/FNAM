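; BP_PickableObject is a world item that goes into the player's inventory when interacted with.
; Its Interaction event casts player 0 to BP_Character and looks up its own class in the Inventory array, which runs parallel to ItemCount.
; It increments the count for a known class or appends the class with a count of one.
; It then destroys itself and calls InventoryUpdateMessage on the character.
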(event EventInteraction
  (bind _self self)
  (bind _returnvalue (Utilities|GetClass _self))
  ;[1 1 1] Pick
  (bind _asbp_character (Utilities|Casting|CastToBP_Character (Game|GetPlayerCharacter 0)))
  (bind _output_get (Variables|Default|SetCharRef _asbp_character))
  (if (Utilities|Array|ContainsItem (Variables|/Game/World/Character/Blueprints/BP_Character.BP_Character_C|GetInventory _output_get) _returnvalue)
    (Utilities|Array|SetArrayElem (Variables|/Game/World/Character/Blueprints/BP_Character.BP_Character_C|GetItemCount _output_get) (Utilities|Array|FindItem (Variables|/Game/World/Character/Blueprints/BP_Character.BP_Character_C|GetInventory _output_get) _returnvalue) (+ (Utilities|Array|Get(acopy) (Variables|/Game/World/Character/Blueprints/BP_Character.BP_Character_C|GetItemCount _output_get) (Utilities|Array|FindItem (Variables|/Game/World/Character/Blueprints/BP_Character.BP_Character_C|GetInventory _output_get) _returnvalue)) 1))
    (else
      (Utilities|Array|Add (Variables|/Game/World/Character/Blueprints/BP_Character.BP_Character_C|GetInventory _output_get) _returnvalue)
      (Utilities|Array|Add (Variables|/Game/World/Character/Blueprints/BP_Character.BP_Character_C|GetItemCount _output_get) 1)))
  (Actor|DestroyActor)
  (Class|BPIInventoryUpdate|InventoryUpdate(Message) _output_get))

(fn ConstructionScript)