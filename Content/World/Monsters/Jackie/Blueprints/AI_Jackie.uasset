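; AI controller for the Jackie monster that runs its behavior tree on possess and drives it from perception updates.
; A sensed target sets Detect and stores the actor as Player in the Blackboard.
; A lost stimulus clears Player, saves the last location, and enables Patrol and Search.
; Timed delays then switch Search to NoticedLocationPatrol and later clear that flag and the saved location.
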(event OnTargetPerceptionUpdated(AIPerception)
  (params (Actor :type Actor%20Object%20Reference) (Stimulus :type AI%20Stimulus%20Structure))
  (bind (_age _expirationage _strength _stimuluslocation _receiverlocation _tag _bsuccessfullysensed) (Utilities|Struct|BreakAIStimulus Stimulus))
  (bind _player (Variables|Default|GetPlayer))
  (bind _noticedlocationvector (Variables|Default|GetNoticedLocationVector))
  (bind _detect (Variables|Default|GetDetect))
  (bind _blackboard (Variables|Default|GetBlackboard))
  (bind _blackboard_2 (Variables|Default|GetBlackboard))
  (bind _search (Variables|Default|GetSearch))
  (bind _noticedlocationpatrol (Variables|Default|GetNoticedLocationPatrol))
  (bind _patrol (Variables|Default|GetPatrol))
  (Variables|Default|SetNoticedLocationPatrolVector _stimuluslocation)
  (if _bsuccessfullysensed
    (Variables|Default|SetBoolSearch false)
    (Variables|Default|SetBoolDetect true)
    (Variables|Default|SetBoolPatrol false)
    (AI|Components|Blackboard|SetValueasBool _blackboard _search (Variables|Default|GetBoolSearch))
    (AI|Components|Blackboard|SetValueasBool _blackboard _patrol (Variables|Default|GetBoolPatrol))
    (AI|Components|Blackboard|SetValueasBool _blackboard _detect (Variables|Default|GetBoolDetect))
    (AI|Components|Blackboard|SetValueasObject _blackboard _player Actor)
    (AI|Components|Blackboard|ClearValue _blackboard_2 _noticedlocationvector)
    (else
      (Variables|Default|SetBoolSearch true)
      (Variables|Default|SetBoolDetect false)
      (Variables|Default|SetBoolPatrol true)
      (AI|Components|Blackboard|SetValueasBool _blackboard _search (Variables|Default|GetBoolSearch))
      (AI|Components|Blackboard|SetValueasBool _blackboard _patrol (Variables|Default|GetBoolPatrol))
      (AI|Components|Blackboard|SetValueasBool _blackboard _detect (Variables|Default|GetBoolDetect))
      (AI|Components|Blackboard|ClearValue _blackboard _player)
      (AI|Components|Blackboard|SetValueasVector _blackboard_2 _noticedlocationvector _stimuluslocation)
      (Utilities|FlowControl|Delay 2.0)
      (Variables|Default|SetBoolSearch false)
      (AI|Components|Blackboard|SetValueasBool _blackboard_2 (Variables|Default|GetSearch) (Variables|Default|GetBoolSearch))
      (Variables|Default|SetBoolNoticedLocationPatrol true)
      (AI|Components|Blackboard|SetValueasBool _blackboard_2 _noticedlocationpatrol (Variables|Default|GetBoolNoticedLocationPatrol))
      (Utilities|FlowControl|Delay (Variables|Default|GetNoticedelay))
      (Variables|Default|SetBoolNoticedLocationPatrol false)
      (AI|Components|Blackboard|SetValueasBool _blackboard_2 _noticedlocationpatrol (Variables|Default|GetBoolNoticedLocationPatrol))
      (AI|Components|Blackboard|ClearValue _blackboard _noticedlocationvector))))

(event EventBeginPlay
  (AI|Components|Blackboard|SetValueasBool (Variables|Default|GetBlackboard) (Variables|Default|GetPatrol) (Variables|Default|GetBoolPatrol)))

(event EventPossess
  (params (PossessedPawn :type Pawn%20Object%20Reference))
  (AI|RunBehaviorTree "/Game/World/Monsters/Jackie/Blueprints/AI/BehaviorTree/BT_Jackie.BT_Jackie"))

(fn ConstructionScript)